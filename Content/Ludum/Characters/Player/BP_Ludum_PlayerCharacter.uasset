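; Player character Blueprint for the Ludum game, handling rifle firing, reloading and the HUD.
; BeginPlay creates the character overlay widget, which health changes update, and refreshes the build wood count.
; Fire input spawns bullets unless the Recoil flag, set during reload, blocks it.
; Reload plays an ALS rifle montage once at a time, spawns a magazine actor at its socket, and destroys it when a timeline finishes.
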(event OnHealthChanged(LudumHealth)
  (params (NewHealth :type Float%20%28single-precision%29))
  (Default|OnHealthChange (Variables|Default|GetStateOverlay) NewHealth 1e+02 1e+01))

(event Input|EnhancedActionEvents|EnhancedInputActionIA_Ludum_Fire
  (params (ActionValue :type Boolean) (ElapsedSeconds :type Float%20%28double-precision%29) (TriggeredSeconds :type Float%20%28double-precision%29) (InputAction :type Input%20Action%20Object%20Reference :default "/Game/Ludum/Input/IA_Ludum_Fire.IA_Ludum_Fire"))
  (:Triggered
    (if (not (Variables|Default|GetRecoil))
      (CallFunction|BSpawnBulletActor true 0.01)
      (Components|Timeline|PlayfromStart (Variables|Default|GetFireTime)))))

(event Input|EnhancedActionEvents|EnhancedInputActionIA_Ludum_Reload
  (params (ActionValue :type Boolean) (ElapsedSeconds :type Float%20%28double-precision%29) (TriggeredSeconds :type Float%20%28double-precision%29) (InputAction :type Input%20Action%20Object%20Reference :default "/Game/Ludum/Input/IA_Ludum_Reload.IA_Ludum_Reload"))
  (:Triggered
    (Variables|Default|SetRecoil true)
    (if true
      (Utilities|FlowControl|DoOnce false :!label _label
        (:Completed
          (Animation|Montage|PlayMontage (Variables|Character|GetMesh) "/Game/Ludum/DataAsset/Animation/ALS_Reloading_Rifle_Montage.ALS_Reloading_Rifle_Montage"
            (:OnCompleted
              (Utilities|FlowControl|Sequence
                (:then_0
                  (goto _label Reset))
                (:then_1
                  (bind _returnvalue (Game|SpawnActorfromClass "/Game/Ludum/DataAsset/weapon/Magazine.Magazine_C" (Transformation|GetSocketTransform (Variables|Default|GetOverlaySkeletalMesh) "magazine" "RTS_World") "Undefined" "MultiplyWithRoot" 0 0 :!label _label_2))
                  (Timeline|RecoilTimeline PlayFromStart
                    (:Finished
                      (Actor|DestroyActor _returnvalue))))
                (:then_2
                  (Variables|Default|SetRecoil false))))
            (:OnNotifyEnd
              (goto _label_2))))))))

(event EventBeginPlay
  (|CallParentFunction)
  (Development|SetHiddeninGame (Variables|Character|GetMesh) false false)
  (bind _returnvalue (UserInterface|CreateWidget "/Game/HUD/WBP_CharacterOverlay.WBP_CharacterOverlay_C"))
  (bind _output_get (Variables|Default|SetStateOverlay _returnvalue))
  (UserInterface|Viewport|AddtoViewport _output_get 0)
  (CallFunction|OnWoodChanged (Variables|Default|GetBuildWood)))

(event Collision|EventActorBeginOverlap
  (params (OtherActor :type Actor%20Object%20Reference)))

(event EventTick
  (params (DeltaSeconds :type Float%20%28single-precision%29))
  (|CallParentFunction DeltaSeconds) ; 此节点被禁用，将不会被调用。\n从引脚连出引线来编译功能。
)

(fn ConstructionScript
  (|CallParentFunction))