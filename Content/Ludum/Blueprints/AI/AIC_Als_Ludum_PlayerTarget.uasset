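; AI controller for Ludum ALS characters that sets the player's pawn as the AI's target.
; On BeginPlay it writes the first player pawn to the TargetActor blackboard key, then copies its AttackRange variable to the key of the same name.
; The target is set once, and no behavior tree is started in this graph.
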(event EventBeginPlay
  (Utilities|FlowControl|Sequence
    (:then_0
      (AI|Components|Blackboard|SetValueasObject (Variables|Default|GetBlackboard) (Utilities|Name|MakeLiteralName "TargetActor") (Game|Player|GetPlayerPawn 0)))
    (:then_1
      (AI|Components|Blackboard|SetValueasFloat (Variables|Default|GetBlackboard) (Utilities|Name|MakeLiteralName "AttackRange") (Variables|Default|GetAttackRange)))))

(fn ConstructionScript
  (|CallParentFunction))