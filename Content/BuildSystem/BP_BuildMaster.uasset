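; BP_BuildMaster is a build-system piece that tracks whether it overlaps another piece or a character and validates snapping.
; Its Box overlap sets OverlayAnother for an ALS character or another BuildMaster's non-box component, so other pieces' box components don't count.
; Each begin overlap overwrites that flag, and any end overlap clears it.
; SnapCheck passes when the given component is in its owning BuildMaster's Floor array and OverlayAnother is false.
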(event OnComponentBeginOverlap(Box)
  (params (OverlappedComponent :type Primitive%20Component%20Object%20Reference) (OtherActor :type Actor%20Object%20Reference) (OtherComp :type Primitive%20Component%20Object%20Reference) (OtherBodyIndex :type Integer) (bFromSweep :type Boolean) (SweepResult :type Hit%20Result%20Structure%20%28by%20ref%29))
  (bind (_asbp_build_master _bsuccess) (Utilities|Casting|CastToBP_BuildMaster OtherActor))
  (Variables|BuildSystem|SetOverlayAnother (or (Math|Boolean|ANDBoolean _bsuccess (!= _asbp_build_master self) (not (.bSuccess (Utilities|Casting|CastToBoxComponent OtherComp)))) (.bSuccess (Utilities|Casting|CastToB_Als_Character OtherActor)))))

(event OnComponentEndOverlap(Box)
  (params (OverlappedComponent :type Primitive%20Component%20Object%20Reference) (OtherActor :type Actor%20Object%20Reference) (OtherComp :type Primitive%20Component%20Object%20Reference) (OtherBodyIndex :type Integer))
  (Variables|BuildSystem|SetOverlayAnother false))

(event EventBeginPlay)

(event Collision|EventActorBeginOverlap
  (params (OtherActor :type Actor%20Object%20Reference)))

(event EventTick
  (params (DeltaSeconds :type Float%20%28single-precision%29)))

(fn ConstructionScript)

(fn SnapCheck
  (params (ItemToFind :type Primitive%20Component%20Object%20Reference))
  (return (and (!= (Utilities|Array|FindItem (Variables|BP_BuildMaster_C|GetFloor (.AsBP%20Build%20Master (Utilities|Casting|CastToBP_BuildMaster (Components|GetOwner ItemToFind)))) ItemToFind) -1) (not (Variables|BuildSystem|GetOverlayAnother)))))