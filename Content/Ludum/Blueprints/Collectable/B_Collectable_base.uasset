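; Base collectable actor that homes in on the player's pawn and is picked up on proximity.
; Tick checks the distance to the player and, while it is within Range, calls FlyToPlayer.
; That function teleports the item closer by a fixed per-frame lerp, so its speed depends on frame rate.
; At close distance it casts to BP_Ludum_PlayerCharacter, calls the empty OnCollected hook, then destroys itself.
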(event EventBeginPlay
  (Variables|默认|SetPlayerActor (Game|Player|GetPlayerPawn 0)))

(event EventTick
  (params (DeltaSeconds :type Float%20%28single-precision%29))
  (if (< (Math|Vector|Distance(Vector) (Transformation|GetActorLocation (Variables|默认|GetPlayerActor)) (Transformation|GetActorLocation)) (Variables|Default|GetRange))
    (Variables|Default|SetbFly true)
    (|FlyToPlayer)))

(fn ConstructionScript)

(fn OnCollected
  (params (PlayerCharacter :type BP%20Ludum%20Player%20Character%20Object%20Reference)))