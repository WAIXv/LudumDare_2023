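; Base damage box actor that acts as a short-lived hitbox for attacks, affecting actors that overlap it.
; On BeginPlay it draws a debug outline of its Box and starts a timer that destroys it after Duration.
; Overlapping actors other than the instigator that have a LudumHealthComponent receive AttackDamage as a health change credited to the instigator.
; Each hit also prints a debug message naming the box, target and damage.
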(event Custom|SelfDestory
  (Actor|DestroyActor))

(event Collision|EventActorBeginOverlap
  (params (OtherActor :type Actor%20Object%20Reference))
  (bind _returnvalue (Actor|GetComponentbyClass OtherActor "/Script/Ludum_2023.LudumHealthComponent"))
  (if (!= OtherActor (Game|GetInstigator))
    (Utilities|IsValid _returnvalue
      (:Is%20Valid
        (Class|LudumHealthComponent|ApplyHealthChange _returnvalue (Game|GetInstigator) (Variables|Default|GetAttackDamage))
        (Development|PrintString (Utilities|String|Append (Utilities|GetDisplayName self) " Attack " (Utilities|GetDisplayName OtherActor) "，Damage：" (Utilities|String|ToString(Float) (Variables|Default|GetAttackDamage))) true true "(R=1.000000,G=0.054287,B=0.000000,A=1.000000)")))))

(event EventBeginPlay
  (bind _box (Variables|Default|GetBox))
  (Rendering|Debug|DrawDebugBox :Center (Transformation|GetWorldLocation _box) :Extent (Variables|/Script/Engine.BoxComponent|GetBoxExtent _box) :Rotation (Transformation|GetWorldRotation _box) :Duration 0.5 :Thickness 3.0)
  (Utilities|Time|SetTimerbyEvent (delegate Custom|SelfDestory) (Variables|Default|GetDuration)))

(fn ConstructionScript)