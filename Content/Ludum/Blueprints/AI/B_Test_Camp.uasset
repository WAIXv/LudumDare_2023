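; A buildable campfire that applies a health change to AI characters within its range and serves as the player's lifeline.
; A looping timer pulses that effect and shrinks the range, while added wood grows it and the light radius tracks it.
; Tick polls a build-finished flag to light the fire, and overlap events register the camp with the player.
; At minimum range the camp explodes, or shows the lose screen and restarts if it is the last one.
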(event OnComponentBeginOverlap(Collision)
  (params (OverlappedComponent :type Primitive%20Component%20Object%20Reference) (OtherActor :type Actor%20Object%20Reference) (OtherComp :type Primitive%20Component%20Object%20Reference) (OtherBodyIndex :type Integer) (bFromSweep :type Boolean) (SweepResult :type Hit%20Result%20Structure%20%28by%20ref%29))
  (bind _asbp_ludum_player_character (Utilities|Casting|CastToBP_Ludum_PlayerCharacter OtherActor))
  (Variables|/Game/Ludum/Characters/Player/BP_Ludum_PlayerCharacter.BP_Ludum_PlayerCharacter_C|SetOverCampActor _asbp_ludum_player_character self)
  (Variables|/Game/Ludum/Characters/Player/BP_Ludum_PlayerCharacter.BP_Ludum_PlayerCharacter_C|SetOverlayCamp _asbp_ludum_player_character true)
  (Development|PrintString "Hello"))

(event OnComponentEndOverlap(Collision)
  (params (OverlappedComponent :type Primitive%20Component%20Object%20Reference) (OtherActor :type Actor%20Object%20Reference) (OtherComp :type Primitive%20Component%20Object%20Reference) (OtherBodyIndex :type Integer))
  (bind _asbp_ludum_player_character (Utilities|Casting|CastToBP_Ludum_PlayerCharacter OtherActor))
  (Variables|/Game/Ludum/Characters/Player/BP_Ludum_PlayerCharacter.BP_Ludum_PlayerCharacter_C|SetOverCampActor _asbp_ludum_player_character self)
  (Variables|/Game/Ludum/Characters/Player/BP_Ludum_PlayerCharacter.BP_Ludum_PlayerCharacter_C|SetOverlayCamp _asbp_ludum_player_character false)
  (Development|PrintString "sadwaw"))

(event Custom|Decrease%20Range
  (bind _outactors (Collision|SphereOverlapActors (Transformation|GetActorLocation) (Variables|Default|GetRange) (Utilities|Array|MakeArray "ObjectTypeQuery3") "/ALS/ALSExtras/AI/B_Als_AICharacter.B_Als_AICharacter_C"))
  (for _array_element _outactors
    (Class|LudumHealthComponent|ApplyHealthChange (Actor|GetComponentbyClass _array_element "/Script/Ludum_2023.LudumHealthComponent") self (Variables|Default|GetDamage)))
  (|销毁))

(event Custom|OnWoodChanged
  (params (NewParam :type Integer))
  (Variables|Default|SetRange (+ (Variables|Default|GetRange) NewParam)))

(event EventBeginPlay
  (Utilities|Time|SetTimerbyEvent (delegate Custom|Decrease%20Range) 3.0 true)
  (Components|Activation|Deactivate (Variables|Default|GetNS_Construction))
  (Rendering|SetVisibility (Variables|Default|GetPointLight) false false)
  (Components|Activation|Deactivate (Variables|Default|GetNS_CampFire))
  (Components|Activation|Deactivate (Variables|Default|GetNS_Explosion)))

(event EventTick
  (params (DeltaSeconds :type Float%20%28single-precision%29))
  (bind _ns_campfire (Variables|Default|GetNS_CampFire))
  (Rendering|Debug|DrawDebugSphere (Transformation|GetActorLocation) (Variables|Default|GetRange) 12 "(R=1.000000,G=0.000000,B=0.023868,A=1.000000)" 0.0)
  (Utilities|FlowControl|Sequence
    (:then_0
      (if (Variables|Default|GetBuildingOver)
        (Variables|Default|SetOver true)
        (Variables|Default|SetBuildingOver false)
        (Rendering|SetVisibility (Variables|Default|GetPointLight) true false)
        (Components|Activation|Activate (Variables|Default|GetNS_Construction) true)
        (Components|Activation|Activate _ns_campfire true)
        (Class|NiagaraComponent|SetAutoDestroy _ns_campfire true)
        (Utilities|FlowControl|Delay 0.85)
        (Components|DestroyComponent (Variables|Default|GetNS_Construction))))
    (:then_1
      (if (Variables|Default|GetOver)
        (Rendering|Lighting|SetAttenuationRadius (Variables|Default|GetPointLight) (Math|Float|MapRangeClamped (Variables|Default|GetRange) 5e+02 0.0 5e+03 0.0))))))

(fn ConstructionScript
  (Variables|Default|SetFloor (Utilities|Array|MakeArray (Variables|Default|GetFloor1) (Variables|Default|GetFloor2) (Variables|Default|GetFloor3) (Variables|Default|GetFloor4))))

(fn GetCurrentRange
  (return (Variables|Default|GetRange)))