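; BP_MonsterC is a monster character Blueprint built on an ALS (Advanced Locomotion System) character parent.
; On BeginPlay it runs the parent logic, then hides the overlay skeletal mesh without propagating to its children.
; Each Tick, after the parent update, it sets actor rotation directly from the movement component's velocity, so the X axis follows the direction of travel with no interpolation.
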(event EventBeginPlay
  (|CallParentFunction)
  (Development|SetHiddeninGame (Variables|Default|GetOverlaySkeletalMesh) true false))

(event Collision|EventActorBeginOverlap
  (params (OtherActor :type Actor%20Object%20Reference)))

(event EventTick
  (params (DeltaSeconds :type Float%20%28single-precision%29))
  (|CallParentFunction DeltaSeconds)
  (Transformation|SetActorRotation (Math|Rotator|MakeRotfromX (Variables|/Script/Engine.MovementComponent|GetVelocity (Variables|Default|GetAlsCharacterMovement)))))

(fn ConstructionScript
  (|CallParentFunction))