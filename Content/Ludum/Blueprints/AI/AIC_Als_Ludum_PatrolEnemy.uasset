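; AI controller for a patrol enemy that feeds a B_Test_Camp target and attack range to its Blackboard.
; BeginPlay stores both keys and caches the target; Tick searches all camps again whenever that cached target becomes invalid.
; GetTargetActor compares each camp's distance from the controller against MinDistance without updating it, so it keeps the last camp within range rather than the nearest.
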(event EventBeginPlay
  (Utilities|FlowControl|Sequence
    (:then_0
      (bind _outactors (Actor|GetAllActorsOfClass "/Game/Ludum/Blueprints/AI/B_Test_Camp.B_Test_Camp_C"))
      (AI|Components|Blackboard|SetValueasObject (Variables|Default|GetBlackboard) (Utilities|Name|MakeLiteralName "TargetActor") (CallFunction|GetTargetActor _outactors))
      (Variables|Default|SetTargetActor1 (CallFunction|GetTargetActor _outactors)))
    (:then_1
      (AI|Components|Blackboard|SetValueasFloat (Variables|Default|GetBlackboard) (Utilities|Name|MakeLiteralName "AttackRange") (Variables|Default|GetAttackRange)))))

(event EventTick
  (params (DeltaSeconds :type Float%20%28single-precision%29))
  (Utilities|IsValid (Variables|Default|GetTargetActor1)
    (:Is%20Not%20Valid
      (bind _outactors (Actor|GetAllActorsOfClass "/Game/Ludum/Blueprints/AI/B_Test_Camp.B_Test_Camp_C"))
      (AI|Components|Blackboard|SetValueasObject (Variables|Default|GetBlackboard) (Utilities|Name|MakeLiteralName "TargetActor") (CallFunction|GetTargetActor _outactors))
      (Variables|Default|SetTargetActor1 (CallFunction|GetTargetActor _outactors)))))

(fn ConstructionScript
  (|CallParentFunction))

(fn GetTargetActor
  (params (CampTargets :type Array%20of%20B%20Test%20Camp%20Object%20References))
  (for _array_element CampTargets
    (if (< (Math|Vector|Distance(Vector) (Transformation|GetActorLocation _array_element) (Transformation|GetActorLocation)) (LocalVariables|GetMinDistance))
      (LocalVariables|SetTargetActor _array_element)))
  (return (LocalVariables|GetTargetActor)))